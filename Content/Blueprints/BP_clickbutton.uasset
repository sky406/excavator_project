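; BP_clickbutton is a button actor that animates its mesh being pressed down and released.
; Custom events ButtonON and ButtonOff each play their own timeline, lerping the SMButton relative location to a slightly lowered offset or back to zero.
; Each lerp starts from the current location rather than a fixed start point.
; It contains no input or overlap logic, so the events must be triggered externally.
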(event `self.buttonON`
  (bind _sm_button (`self.SM_button`))
  (bind (_direction _button_down) (`Timeline|button click on`)
    (:`Update`
      (`SceneComponent.K2_SetRelativeLocation` _sm_button (`KismetMathLibrary.VLerp` (`SceneComponent.RelativeLocation` _sm_button) (0.0 0.0 -0.150066) _button_down) false false))))

(event `self.buttonOff`
  (bind _sm_button (`self.SM_button`))
  (bind (_direction _button_click_off) (`Timeline|buttonclick off`)
    (:`Update`
      (`SceneComponent.K2_SetRelativeLocation` _sm_button (`KismetMathLibrary.VLerp` (`SceneComponent.RelativeLocation` _sm_button) (0.0 0.0 0.0) _button_click_off) false false))))

(fn `UserConstructionScript`
  (`parent.UserConstructionScript`))