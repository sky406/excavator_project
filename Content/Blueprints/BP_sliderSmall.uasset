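; BP_sliderSmall is the small variant of a slider, configuring logic inherited from its parent Blueprint.
; On BeginPlay it runs the parent logic, then assigns the small knob component as the slider component and sets symmetric minimum and maximum travel distances.
; It adds no movement logic of its own: Tick and overlap events are disabled, and the construction script only calls the parent.
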(event `self.ReceiveBeginPlay`
  (`parent.ReceiveBeginPlay`)
  (set `self.sliderComponent` (`self.SM_slider_knob_small`))
  (set `self.maxDist` 12.0)
  (set `self.minDist` -12.0))

(fn `UserConstructionScript`
  (`parent.UserConstructionScript`))