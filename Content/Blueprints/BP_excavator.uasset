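; BP_excavator is a drivable excavator actor that exposes events for turning, arm control and lighting.
; Opposing throttle inputs yaw the actor, while track movement and throttle processing are empty stubs.
; Stick input yaws RotatorCube and drives forearm, arm and bucket Control Rig controls on ExcaTop, mapped to the skeletal mesh, with clamped arm and bucket angles.
; A light event sets intensity, color and temperature on four front lights.
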(event `self.ReceiveBeginPlay`
  (set `self.lights` (`|MakeArray` (`self.frontLight`) (`self.frontLight1`) (`self.frontLight2`) (`self.frontLight3`))))

(event `self.ReceiveTick`
  (params (DeltaSeconds :type "Float (single-precision)")))

(event `rotate excavator`
  (params (`left throttle` :type "Float (double-precision)") (`right throttle` :type "Float (double-precision)"))
  (bind _rotation_speed (`self.rotation speed`))
  (`self.K2_AddActorWorldRotation` (`KismetMathLibrary.MakeRotator` 0.0 0.0 (+ (* `left throttle` _rotation_speed) (* _rotation_speed (* `right throttle` -1.0))))))

(event `changeLightstate`
  (params (on :type Boolean) (color :type "LinearColor Structure") (`color temperature` :type "Float (double-precision)"))
  (for _array_element (`self.lights`)
    (if on
      (`LightComponent.SetIntensity` _array_element (`self.lightIntensity`))
      (else
        (`LightComponent.SetIntensity` _array_element 0.0)))
    (`LightComponent.SetLightColor` _array_element color true)
    (`LightComponent.SetTemperature` _array_element `color temperature`)))

(event `self.excaTop.OnPreInitializeDelegate`
  (params (Component :type "ControlRigComponent Object Reference"))
  ; setup
  (`ControlRigComponent.AddMappedCompleteSkeletalMesh` Component (`self.excavator top`) "Output")
  (`ActorComponent.Activate` (`self.excaTop`) false)
  (`ActorComponent.Activate` Component false))

(event `armUpdate`
  (params (leftstickPos :type "Vector2D Structure") (rightstickPos :type "Vector2D Structure"))
  (bind (_x _y) (`KismetMathLibrary.BreakVector2D` rightstickPos))
  (bind (_x_2 _y_2) (`KismetMathLibrary.BreakVector2D` leftstickPos))
  (bind _excatop (`self.excaTop`))
  (bind _excatop_2 (`self.excaTop`))
  (bind _excatop_3 (`self.excaTop`))
  (bind (_returnvalue_roll _returnvalue_pitch _returnvalue_yaw) (`KismetMathLibrary.BreakRotator` (`ControlRigComponent.GetControlRotator` _excatop "bucket_ctrl" "LocalSpace")))
  (bind (_returnvalue_roll_2 _returnvalue_pitch_2 _returnvalue_yaw_2) (`KismetMathLibrary.BreakRotator` (`ControlRigComponent.GetControlRotator` _excatop_3 "foreArm_ctrl" "LocalSpace")))
  (bind (_returnvalue_roll_3 _returnvalue_pitch_3 _returnvalue_yaw_3) (`KismetMathLibrary.BreakRotator` (`ControlRigComponent.GetControlRotator` _excatop_2 "arm_ctrl" "LocalSpace")))
  ; left stick
  (`ControlRigComponent.SetControlRotator` _excatop_3 "foreArm_ctrl" (`KismetMathLibrary.MakeRotator` (`KismetMathLibrary.FClamp` (+ (* _x_2 (`self.armSpeed`) -1.0) _returnvalue_roll_2) -75.0 0.0) _returnvalue_pitch_2 _returnvalue_yaw_2) "LocalSpace")
  (`SceneComponent.K2_AddRelativeRotation` (`self.rotator cube`) (`KismetMathLibrary.MakeRotator` 0.0 0.0 (* _y_2 (`self.rotateSpeed`))) false false)
  ; right stick
  (`ControlRigComponent.SetControlRotator` _excatop "bucket_ctrl" (`KismetMathLibrary.MakeRotator` (`KismetMathLibrary.FClamp` (+ (* _x (`self.armSpeed`)) _returnvalue_roll) -10.0 90.0) _returnvalue_pitch _returnvalue_yaw) "LocalSpace")
  (`ControlRigComponent.SetControlRotator` _excatop_2 "arm_ctrl" (`KismetMathLibrary.MakeRotator` (`KismetMathLibrary.FClamp` (+ (* _y (`self.armSpeed`)) _returnvalue_roll_3) -50.0 20.0) _returnvalue_pitch_3 _returnvalue_yaw_3) "LocalSpace"))

(event `move tracks`
  (params (leftSpeed :type "Float (double-precision)") (rightSpeed :type "Float (double-precision)")))

(fn `processThrottleInputs`
  (params (`left input` :type "Float (double-precision)") (`right input` :type "Float (double-precision)")))

(fn `UserConstructionScript`)