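; BP_joystick is an interactive joystick that tilts its Sphere component in response to signals from its parent class.
; While signalled, it sets clamped roll and pitch from DistanceFromStart and StickSpeed, and stops the return timeline.
; After the signal ends, Tick restarts the BackToZero timeline every frame to lerp the stick back to centre.
; Directional events are stubs, with only up printing a debug string.
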(event `joystick up`
  (`KismetSystemLibrary.PrintString` "up"))

(event `self.ReceiveTick`
  (params (DeltaSeconds :type "Float (single-precision)"))
  (bind _sphere (`self.Sphere`))
  (`parent.ReceiveTick` DeltaSeconds)
  ; reset stick position
  (if (not (`self.stickHeld`))
    (bind (_direction _return_to_zero) (`Timeline|back to zero` :!via `PlayFromStart` :!label _label)
      (:`Update`
        (`SceneComponent.K2_SetRelativeRotation` _sphere (`KismetMathLibrary.RLerp` (`SceneComponent.RelativeRotation` _sphere) (struct) _return_to_zero) false false)))))

(event `joystick down`)

(event `joystick left`)

(event `joystick right`)

(event `self.signal recieved`
  (params (`mouse position` :type "Vector Structure") (`mouse delta` :type "Vector Structure"))
  (bind (_distancefromstart_x _distancefromstart_y _distancefromstart_z) (`KismetMathLibrary.BreakVector` (`self.distanceFromStart`)))
  (bind _stickspeed (`self.stickSpeed`))
  (`parent.signal recieved` `mouse position` (0.0 0.0 0.0))
  ; stick manipulation
  (set `self.stickHeld` true)
  (`SceneComponent.K2_SetRelativeRotation` (`self.Sphere`) (`KismetMathLibrary.MakeRotator` (`KismetMathLibrary.FClamp` (* _distancefromstart_y _stickspeed) -50.0 50.0) (`KismetMathLibrary.FClamp` (* (* _stickspeed _distancefromstart_z) -1.0) -50.0 50.0)) false false)
  (goto _label :!via `Stop`))

(event `self.signal end`
  (`parent.signal end`)
  (set `self.stickHeld` false))

(fn `UserConstructionScript`
  (`parent.UserConstructionScript`))