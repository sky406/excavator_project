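; BP_sliderBig is a large slider control that carries two smaller offset sliders, left and right, as child actors.
; BeginPlay binds the knob mesh and sets its travel limits.
; Mouse input runs the parent handling, then forwards the same delta to both child sliders so they move along with it.
; Tick stores each child's level relative to the main level as LeftOffset and RightOffset.
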(event `self.ReceiveBeginPlay`
  (`parent.ReceiveBeginPlay`)
  (set `self.sliderComponent` (`self.SM_slider_knob1`))
  (set `self.maxDist` 12.0)
  (set `self.minDist` -12.0))

(event `self.ReceiveTick`
  (params (DeltaSeconds :type "Float (single-precision)"))
  (`parent.ReceiveTick` DeltaSeconds)
  (bind _as_bp_slider (cast `/Game/Blueprints/_BP_slider` (`ChildActorComponent.ChildActor` (`self.offset slider R`))))
  (set `self.right offset` (- (`/Game/Blueprints/_BP_slider.sliderLevel` _as_bp_slider) (`self.sliderLevel`)))
  (bind _as_bp_slider_2 (cast `/Game/Blueprints/_BP_slider` (`ChildActorComponent.ChildActor` (`self.offest slider L`))))
  (set `self.left offset` (- (`/Game/Blueprints/_BP_slider.sliderLevel` _as_bp_slider_2) (`self.sliderLevel`))))

(event `/Game/Blueprints/_BP_reciever.signal recieved`
  (params (`mouse position` :type "Vector Structure") (`mouse delta` :type "Vector Structure"))
  (`parent.signal recieved` `mouse position` `mouse delta`)
  (bind _as_bp_slider (cast `/Game/Blueprints/_BP_slider` (`ChildActorComponent.ChildActor` (`self.offset slider R`))))
  (`self.moveSlider` _as_bp_slider `mouse delta`)
  (bind _as_bp_slider_2 (cast `/Game/Blueprints/_BP_slider` (`ChildActorComponent.ChildActor` (`self.offest slider L`))))
  (`self.moveSlider` _as_bp_slider_2 `mouse delta`))

(fn `UserConstructionScript`
  (`parent.UserConstructionScript`))