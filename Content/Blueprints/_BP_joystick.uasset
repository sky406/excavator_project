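; Interactive joystick Blueprint that turns mouse-driven signals from its parent class into lever tilt and directional input percentages.
; While signalled, it sets clamped roll and pitch from DistanceFromStart and StickSpeed, and stops the return timeline.
; When not held, Tick restarts the BackToZero timeline, which lerps the lever toward its resting angle.
; Both paths convert rotation into left, right, forward and backward percentages; BeginPlay clears LeverComponent, marked for removal.
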(event `self.ReceiveBeginPlay`
  (`parent.ReceiveBeginPlay`)
  ; remove later
  (set `self.leverComponent` null))

(event `self.ReceiveTick`
  (params (DeltaSeconds :type "Float (single-precision)"))
  (bind _levercomponent (`self.leverComponent`))
  (`parent.ReceiveTick` DeltaSeconds)
  ; reset stick position
  (if (not (`self.stickHeld`))
    (bind (_direction _return_to_zero) (`Timeline|back to zero` :!via `PlayFromStart` :!label _label)
      (:`Update`
        (`SceneComponent.K2_SetRelativeRotation` _levercomponent (`KismetMathLibrary.RLerp` (`SceneComponent.RelativeRotation` _levercomponent) (`self.restingAngle`) _return_to_zero) false false)
        (`self.mark rotation`)))))

(event `self.signal recieved`
  (params (`mouse position` :type "Vector Structure") (`mouse delta` :type "Vector Structure"))
  (`parent.signal recieved` `mouse position` (0.0 0.0 0.0))
  (`self.rotate lever` (`self.leverComponent`) `mouse delta`)
  (`self.mark rotation`)
  (goto _label :!via `Stop`))

(event `mark rotation`
  (bind (_relativerotation_roll _relativerotation_pitch) (`KismetMathLibrary.BreakRotator` (`SceneComponent.RelativeRotation` (`self.leverComponent`))))
  (if (< _relativerotation_roll 0.0)
    (set `self.leftPercent` (/ (* _relativerotation_roll -1.0) (* (`self.minRoll`) -1.0)))
    (set `self.rightPercent` 0.0)
    (else
      (set `self.rightPercent` (/ _relativerotation_roll (`self.maxRoll`)))
      (set `self.leftPercent` 0.0)))
  (if (< _relativerotation_pitch 0.0)
    (set `self.forward Percent` (/ (* _relativerotation_pitch -1.0) (* (`self.minPitch`) -1.0)))
    (set `self.backwardPercent` 0.0)
    (else
      (set `self.backwardPercent` (/ _relativerotation_pitch (`self.MaxPitch`)))
      (set `self.forward Percent` 0.0))))

(event `self.signal end`
  (`parent.signal end`)
  (set `self.stickHeld` false))

(fn `rotate lever`
  (params (rotatedComponent :type "SceneComponent Object Reference") (`input vector` :type "Vector Structure"))
  (bind (_distancefromstart_x _distancefromstart_y _distancefromstart_z) (`KismetMathLibrary.BreakVector` (`self.distanceFromStart`)))
  (bind _stickspeed (`self.stickSpeed`))
  ; stick manipulation
  (set `self.stickHeld` true)
  (`SceneComponent.K2_SetRelativeRotation` rotatedComponent (`KismetMathLibrary.MakeRotator` (`KismetMathLibrary.FClamp` (* (* _distancefromstart_y _stickspeed) 1.0) (`self.minRoll`) (`self.maxRoll`)) (`KismetMathLibrary.FClamp` (* (* _stickspeed _distancefromstart_z) -1.0) (`self.minPitch`) (`self.MaxPitch`))) false false))

(fn `UserConstructionScript`
  (`parent.UserConstructionScript`))