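; BP_rotator is a signal-driven actor that rotates with mouse movement.
; On each received signal, it reads the player controller's mouse delta and applies world pitch from vertical and yaw from horizontal movement, inverted and scaled by RotationSpeed.
; Rotation axes are fixed in world space, so author notes flag that controls only work with the camera facing X.
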(event `self.signal recieved`
  (params (`mouse position` :type "Vector Structure") (`mouse delta` :type "Vector Structure"))
  (bind _returnvalue (* (`self.rotationSpeed`) -1.0))
  (`parent.signal recieved` `mouse position` (0.0 0.0 0.0))
  (bind _asplayer_controller (cast `PlayerController` (`GameplayStatics.GetPlayerController` 0)))
  (bind (_deltax _deltay) (`PlayerController.GetInputMouseDelta` _asplayer_controller))
  ; note to self this entire thing only works as long as the camera is facing the x drection
  (`self.K2_AddActorWorldRotation` (`KismetMathLibrary.MakeRotator` 0.0 (* _deltay _returnvalue) (* _deltax _returnvalue))) ; note to self make this relative to the camera angle
  (`KismetSystemLibrary.PrintString` ""))

(event `self.signal end`
  (`parent.signal end`))

(fn `UserConstructionScript`
  (`parent.UserConstructionScript`))