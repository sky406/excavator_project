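; Player character Blueprint with tank-style controls driven by Enhanced Input.
; On BeginPlay it adds the BP_inputs mapping context to the local player's input subsystem.
; IA_Move drives movement along the actor's forward vector and prints the input value and velocity for debugging.
; IA_rotate adds input scaled by TurnSpeed to the controller's yaw, without delta-time scaling.
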(event `self.ReceiveBeginPlay`
  ; add inputs
  (bind _asplayer_controller (cast `PlayerController` (`GameplayStatics.GetPlayerController` 0)))
  (bind _returnvalue (pcsubsystem `EnhancedInputLocalPlayerSubsystem` _asplayer_controller))
  (`/Engine/EditorBlueprintResources/StandardMacros.IsValid` _returnvalue
    (:`Is Valid`
      (`EnhancedInputSubsystemInterface.AddMappingContext` _returnvalue "/Game/Blueprints/inputs/BP_inputs.BP_inputs" 0 (struct)))))

(event `EnhancedInput|/Game/Blueprints/inputs/input_Actions/IA_Move`
  (params (ActionValue :type "Float (double-precision)") (ElapsedSeconds :type "Float (double-precision)") (TriggeredSeconds :type "Float (double-precision)") (InputAction :type "InputAction Object Reference" :default "/Game/Blueprints/inputs/input_Actions/IA_Move.IA_Move"))
  ; move forward and back
  (:`Triggered`
    (`self.AddMovementInput` (`KismetMathLibrary.GetForwardVector` (`self.K2_GetActorRotation`)) ActionValue)
    (`KismetSystemLibrary.PrintString` (`KismetStringLibrary.Conv_DoubleToString` ActionValue))
    (`KismetSystemLibrary.PrintString` (`KismetStringLibrary.Conv_VectorToString` (`CharacterMovementComponent.GetLastUpdateVelocity` (`self.CharacterMovement`))))))

(event `EnhancedInput|/Game/Blueprints/inputs/input_Actions/IA_rotate`
  (params (ActionValue :type "Float (double-precision)") (ElapsedSeconds :type "Float (double-precision)") (TriggeredSeconds :type "Float (double-precision)") (InputAction :type "InputAction Object Reference" :default "/Game/Blueprints/inputs/input_Actions/IA_rotate.IA_rotate"))
  (bind _returnvalue (`GameplayStatics.GetPlayerController` 0))
  (bind (_returnvalue_roll _returnvalue_pitch _returnvalue_yaw) (`KismetMathLibrary.BreakRotator` (`Controller.GetControlRotation` _returnvalue)))
  ; tank turning
  (:`Triggered`
    (`Controller.SetControlRotation` _returnvalue (`KismetMathLibrary.MakeRotator` _returnvalue_roll _returnvalue_pitch (+ _returnvalue_yaw (* ActionValue (`self.turnSpeed`)))))))

(fn `UserConstructionScript`)