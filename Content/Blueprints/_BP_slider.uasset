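; Slider actor that moves a component along its local Y axis from mouse-drag signals and exposes the result as SliderLevel.
; SignalRecieved forwards a zeroed delta to the parent, then MoveSlider scales mouse Y by Sliderspeed and clamps the new position between MinDist and MaxDist.
; Each move calls updatedposition, which normalizes each side of zero against its own limit into a signed level rounded to one decimal.
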(event `self.signal recieved`
  (params (`mouse position` :type "Vector Structure") (`mouse delta` :type "Vector Structure"))
  (`parent.signal recieved` `mouse position` (0.0 0.0 0.0))
  (`self.moveSlider` `mouse delta`))

(event `self.signal end`
  (`parent.signal end`))

(event `updated position`
  (bind (_relativelocation_x _relativelocation_y) (`KismetMathLibrary.BreakVector` (`SceneComponent.RelativeLocation` (`self.sliderComponent`))))
  ; set slider level
  (if (> _relativelocation_y 0.0)
    (bind _rounded (`self.round to 1 decimal` (/ _relativelocation_y (`self.maxDist`))))
    (set `self.sliderLevel` _rounded)
    (else
      (bind _rounded_2 (`self.round to 1 decimal` (* (/ _relativelocation_y (`self.minDist`)) -1.0)))
      (set `self.sliderLevel` _rounded_2))))

(event `setSliderPos`)

(fn `moveSlider`
  (params (inputVector :type "Vector Structure"))
  (bind (_relativelocation_x _relativelocation_y _relativelocation_z) (`KismetMathLibrary.BreakVector` (`SceneComponent.RelativeLocation` (`self.sliderComponent`))))
  ; move slider
  (bind _rounded (`self.round to 1 decimal` (+ (* (`self.sliderspeed`) (+ (.y inputVector) 0.0)) _relativelocation_y)))
  (`SceneComponent.K2_SetRelativeLocation` (`self.sliderComponent`) (`KismetMathLibrary.MakeVector` _relativelocation_x (`KismetMathLibrary.FClamp` _rounded (`self.minDist`) (`self.maxDist`)) _relativelocation_z) false false)
  (`self.updated position`))

(fn `round to 1 decimal`
  (params (float :type "Float (double-precision)"))
  (returns (rounded :type "Float (double-precision)"))
  (return (/ (`KismetMathLibrary.Conv_IntToDouble` (`KismetMathLibrary.Round` (* float 10.0))) 10.0)))

(fn `UserConstructionScript`
  (`parent.UserConstructionScript`))