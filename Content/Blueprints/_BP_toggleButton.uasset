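; Base toggle button Blueprint that switches between on and off in response to signals inherited from its parent class.
; When a signal ends, it flips the Toggled flag and fires a state change that calls either ButtonON or ButtonOff.
; Both of those events are empty here, so this asset defines no on/off behavior itself.
; Received signals pass the mouse position to the parent with a zero mouse delta.
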(event `self.signal end`
  (`parent.signal end`)
  (set `self.toggled` (not (`self.toggled`)))
  (`self.stateChanged`))

(event `self.signal recieved`
  (params (`mouse position` :type "Vector Structure") (`mouse delta` :type "Vector Structure"))
  (`parent.signal recieved` `mouse position` (0.0 0.0 0.0)))

(event `stateChanged`
  (if (`self.toggled`)
    (`self.buttonON`)
    (else
      (`self.buttonOff`))))

(event `buttonON`)

(event `buttonOff`)

(fn `UserConstructionScript`
  (`parent.UserConstructionScript`))