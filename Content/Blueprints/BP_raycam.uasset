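; BP_raycam is the player's excavator control rig, operating child-actor joysticks, throttles, sliders and a toggle button with the mouse.
; A click line-traces from the cursor to latch a _BP_reciever, which gets mouse position and delta until release.
; Tick reads the controls, feeding throttles into excavator rotation and rig movement, and the toggle into its light.
; Offset sliders set the throttles' resting angles; stick positions are only stored.
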(event `self.ReceiveBeginPlay`
  ; temporary(remove later)
  (bind _returnvalue (`|CreateWidget` "/Game/Blueprints/debugTools/BP_control_info.BP_control_info_C"))
  (`UserWidget.AddToViewport` _returnvalue 0)
  (bind _asbp_excavator (cast `/Game/Blueprints/BP_excavator` (`ChildActorComponent.ChildActor` (`self.excavator`))))
  (`/Game/Blueprints/BP_excavator.changeLightstate` _asbp_excavator true (struct :`R` 1.0 :`G` 0.259195 :`B` 0.239298 :`A` 1.0) 220.0))

(event `EnhancedInput|/Game/Blueprints/inputs/input_Actions/IA_Click`
  (params (ActionValue :type Boolean) (ElapsedSeconds :type "Float (double-precision)") (TriggeredSeconds :type "Float (double-precision)") (InputAction :type "InputAction Object Reference" :default "/Game/Blueprints/inputs/input_Actions/IA_Click.IA_Click"))
  (bind (_deltax _deltay) (`PlayerController.GetInputMouseDelta` (`GameplayStatics.GetPlayerController` 0)))
  (bind (_worldlocation _worlddirection) (`PlayerController.DeprojectMousePositionToWorld` (`GameplayStatics.GetPlayerController` 0)))
  (:`Triggered`
    ; broadcast mouse movement to controller
    (if (`self.controller_selected`)
      (bind _as_bp_reciever (cast `/Game/Blueprints/_BP_reciever` (`self.last connected`)))
      (`/Game/Blueprints/_BP_reciever.signal recieved` _as_bp_reciever _worldlocation (`KismetMathLibrary.MakeVector` _deltax _deltay))))
  (:`Started`
    ; connecting to the controllers
    (bind _outhit (`KismetSystemLibrary.LineTraceSingle` _worldlocation (+ _worldlocation (* _worlddirection 15000.0)) "TraceTypeQuery1"))
    (bind (_bblockinghit _binitialoverlap _time _distance _location _impactpoint _normal _impactnormal _physmat _hitactor) (`GameplayStatics.BreakHitResult` _outhit))
    (if (`KismetMathLibrary.ClassIsChildOf` (`GameplayStatics.GetObjectClass` _hitactor) "/Game/Blueprints/_BP_reciever._BP_reciever_C")
      (`/Engine/EditorBlueprintResources/StandardMacros.DoOnce` false :!label _label
        (:`Completed`
          (set `self.controller_selected` true)
          (bind _output_get (set `self.last connected` _hitactor))
          (bind _as_bp_reciever_2 (cast `/Game/Blueprints/_BP_reciever` _output_get))
          (`/Game/Blueprints/_BP_reciever.signal recieved` _as_bp_reciever_2 _worldlocation (0.0 0.0 0.0))))))
  (:`Canceled`
    ; reset after player releases
    (if (`KismetMathLibrary.ClassIsChildOf` (`GameplayStatics.GetObjectClass` (`self.last connected`)) "/Game/Blueprints/_BP_reciever._BP_reciever_C") :!label _label_2
      (bind _as_bp_reciever_3 (cast `/Game/Blueprints/_BP_reciever` (`self.last connected`)))
      (`/Game/Blueprints/_BP_reciever.signal end` _as_bp_reciever_3)
      (set `self.controller_selected` false)
      (goto _label :!via `Reset`)))
  (:`Completed`
    (goto _label_2)))

(event `self.ReceiveTick`
  (params (DeltaSeconds :type "Float (single-precision)"))
  (bind (_forward_percent _backwardpercent _leftpercent _rightpercent) (`self.getStickData` (`ChildActorComponent.ChildActor` (`self.stick L`))))
  (set `self.leftStickPos` (`KismetMathLibrary.MakeVector2D` (- _forward_percent _backwardpercent) (- _rightpercent _leftpercent)))
  (bind (_forward_percent_2 _backwardpercent_2 _leftpercent_2 _rightpercent_2) (`self.getStickData` (`ChildActorComponent.ChildActor` (`self.stick R`))))
  (set `self.rightStickPos` (`KismetMathLibrary.MakeVector2D` (- _forward_percent_2 _backwardpercent_2) (- _rightpercent_2 _leftpercent_2)))
  (bind (_forward_percent_3 _backwardpercent_3) (`self.getStickData` (`ChildActorComponent.ChildActor` (`self.ThrottleL`))))
  (set `self.leftThrottleVar` (- _forward_percent_3 _backwardpercent_3))
  (bind (_forward_percent_4 _backwardpercent_4) (`self.getStickData` (`ChildActorComponent.ChildActor` (`self.ThrottleR`))))
  (set `self.rightThrottleVar` (- _forward_percent_4 _backwardpercent_4))
  (bind _asbp_excavator (cast `/Game/Blueprints/BP_excavator` (`ChildActorComponent.ChildActor` (`self.excavator`))))
  ; excavator controls
  (`/Game/Blueprints/BP_excavator.rotate excavator` _asbp_excavator (`self.leftThrottleVar`) (`self.rightThrottleVar`))
  (`self.K2_AddActorWorldOffset` (* (`SceneComponent.GetRightVector` (`/Game/Blueprints/BP_excavator.excavator base` _asbp_excavator)) (* (`self.excavator speed`) (`KismetMathLibrary.FClamp` (+ (`self.leftThrottleVar`) (`self.rightThrottleVar`)) -1.0))))
  (bind _asbp_slider_big (cast `/Game/Blueprints/BP_sliderBig` (`ChildActorComponent.ChildActor` (`self.TsLIDER`))))
  (bind _as_bp_slider (cast `/Game/Blueprints/_BP_slider` (`ChildActorComponent.ChildActor` (`/Game/Blueprints/BP_sliderBig.offest slider L` _asbp_slider_big))))
  (set `self.leftOffsetSliderLevel` (`/Game/Blueprints/_BP_slider.sliderLevel` _as_bp_slider))
  (bind _as_bp_slider_2 (cast `/Game/Blueprints/_BP_slider` (`ChildActorComponent.ChildActor` (`/Game/Blueprints/BP_sliderBig.offset slider R` _asbp_slider_big))))
  (set `self.rightOffsetSliderLevel` (`/Game/Blueprints/_BP_slider.sliderLevel` _as_bp_slider_2))
  (bind _as_bp_joystick (cast `/Game/Blueprints/_BP_joystick` (`ChildActorComponent.ChildActor` (`self.ThrottleL`))))
  (bind _pitch (`self.joystickAngleConvert` _as_bp_joystick (`self.leftOffsetSliderLevel`)))
  (set `/Game/Blueprints/_BP_joystick.restingAngle` (`KismetMathLibrary.MakeRotator` 0.0 _pitch) _as_bp_joystick)
  (bind _as_bp_joystick_2 (cast `/Game/Blueprints/_BP_joystick` (`ChildActorComponent.ChildActor` (`self.ThrottleR`))))
  (bind _pitch_2 (`self.joystickAngleConvert` _as_bp_joystick_2 (`self.rightOffsetSliderLevel`)))
  (set `/Game/Blueprints/_BP_joystick.restingAngle` (`KismetMathLibrary.MakeRotator` 0.0 _pitch_2) _as_bp_joystick_2)
  (bind _as_bp_toggle_button (cast `/Game/Blueprints/_BP_toggleButton` (`ChildActorComponent.ChildActor` (`self.button`))))
  (`/Game/Blueprints/BP_excavator.changeLightstate` _asbp_excavator (`/Game/Blueprints/_BP_toggleButton.toggled` _as_bp_toggle_button) (struct :`R` 1.0 :`G` 0.69197 :`B` 0.335289 :`A` 1.0) 3300.0))

(fn `getSliderData`
  (params (slider :type "Object Object Reference"))
  (returns (sliderLevel :type "Float (double-precision)") (`Relative Location Y` :type "Float (double-precision)") (`left offset` :type "Float (double-precision)") (`right offset` :type "Float (double-precision)"))
  (bind _asbp_slider_big (cast `/Game/Blueprints/BP_sliderBig` slider))
  (bind (_relativelocation_x _relativelocation_y) (`KismetMathLibrary.BreakVector` (`SceneComponent.RelativeLocation` (`/Game/Blueprints/_BP_slider.sliderComponent` _asbp_slider_big))))
  (return (`/Game/Blueprints/_BP_slider.sliderLevel` _asbp_slider_big) _relativelocation_y (`/Game/Blueprints/BP_sliderBig.right offset` _asbp_slider_big) (`/Game/Blueprints/BP_sliderBig.left offset` _asbp_slider_big)))

(fn `getStickData`
  (params (joystickdata :type "Object Object Reference"))
  (returns (`forward Percent` :type "Float (double-precision)") (backwardPercent :type "Float (double-precision)") (leftPercent :type "Float (double-precision)") (rightPercent :type "Float (double-precision)"))
  (bind _as_bp_joystick (cast `/Game/Blueprints/_BP_joystick` joystickdata))
  (return (`/Game/Blueprints/_BP_joystick.forward Percent` _as_bp_joystick) (`/Game/Blueprints/_BP_joystick.backwardPercent` _as_bp_joystick) (`/Game/Blueprints/_BP_joystick.leftPercent` _as_bp_joystick) (`/Game/Blueprints/_BP_joystick.rightPercent` _as_bp_joystick)))

(fn `joystickAngleConvert`
  (params (joystick :type "/Game/Blueprints/_BP_joystick Object Reference") (percent :type "Float (double-precision)"))
  (returns (pitch :type "Float (double-precision)"))
  (if (> percent 0.0)
    (bind _result (`/Engine/EditorBlueprintResources/StandardMacros.NegateFloat` (* (`/Game/Blueprints/_BP_joystick.MaxPitch` joystick) percent))
      (:`  `
        (return _result)))
    (else
      (return (* (`/Game/Blueprints/_BP_joystick.minPitch` joystick) percent)))))

(fn `UserConstructionScript`)